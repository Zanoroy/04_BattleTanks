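; Player-controllable tank Blueprint that routes input to its driving, firing and camera components.
; BeginPlay hands the left and right tracks to TankMovement, and the barrel and turret to TankAiming.
; Drive axes pass movement intent to TankMovement, while the Fire press triggers TankAiming's projectile.
; Aim axes orbit the camera using delta-time-scaled local rotations, with yaw on the azimuth gimbal and pitch on the spring arm.
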(event EventBeginPlay
  (Class|TankMovementComponent|Initialise (Variables|Default|GetTankMovement) (Variables|Default|GetLeftTrack) (Variables|Default|GetRightTrack))
  (Class|TankAimingComponent|Initalise (Variables|Default|GetTankAiming) (Variables|Default|GetBarrel) (Variables|Default|GetTankTurret)))

(event Input|ActionEvents|InputActionFire
  (params (Key :type Key%20Structure))
  (:Pressed
    (Class|TankAimingComponent|FireProjectile (Variables|Default|GetTankAiming))))

(event Input|AxisEvents|InputAxisAimAzimuth
  (params (AxisValue :type Float%20%28single-precision%29))
  ;[1 1 1] Camera Binding
  (Transformation|AddLocalRotation (Variables|Default|GetAzimuth%20Gimbol) (Math|Rotator|MakeRotator 0.0 0.0 (* AxisValue (Utilities|Time|GetWorldDeltaSeconds) 1e+02)) false false))

(event Input|AxisEvents|InputAxisTurnClockwise
  (params (AxisValue :type Float%20%28single-precision%29))
  ;[1 1 1] Driving Tracks
  (Class|TankMovementComponent|IntendTurnClockwise (Variables|Default|GetTankMovement) AxisValue))

(event Input|AxisEvents|InputAxisAimZenith
  (params (AxisValue :type Float%20%28single-precision%29))
  ;[1 1 1] Zenith Rotation
  (Transformation|AddLocalRotation (Variables|Default|GetSpringArm) (Math|Rotator|MakeRotator 0.0 (* AxisValue (Utilities|Time|GetWorldDeltaSeconds) 1e+02) 0.0) false false))

(event Input|AxisEvents|InputAxisMoveForward
  (params (AxisValue :type Float%20%28single-precision%29))
  ;[1 1 1] Driving Tracks
  (Class|TankMovementComponent|IntendMovementFoward (Variables|Default|GetTankMovement) AxisValue))

(fn ConstructionScript)